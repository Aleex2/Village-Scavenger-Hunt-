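; BP_Class is a first-person style player character with movement, look, jump, interaction and pause input.
; Each tick, a camera-forward Visibility line trace stores the hit actor in ObjectLookingAt.
; Interact casts that actor to Master_Interact and calls InteractWithObject.
; P and Escape share a FlipFlop that toggles game pause, creating and adding a new Ui_Pause widget on every press.
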(event EventTick
  (params (DeltaSeconds :type Float%20%28single-precision%29))
  (bind _returnvalue (Game|GetPlayerCameraManager 0))
  (bind _returnvalue_2 (Transformation|GetActorLocation _returnvalue))
  (bind (_outhit _returnvalue_3) (Collision|LineTraceByChannel _returnvalue_2 (+ _returnvalue_2 (* (Transformation|GetActorForwardVector _returnvalue) (Variables|Default|GetDistanceForLooking))) "TraceTypeQuery1" false 0 "None"))
  (if _returnvalue_3
    (Variables|Default|SetObjectLookingAt (.HitActor (Collision|BreakHitResult _outhit)))
    (else
      (Variables|Default|SetObjectLookingAt 0))))

(event Input|ActionEvents|InputActionJump
  (params (Key :type Key%20Structure :default "None"))
  (:Pressed
    (Character|Jump)))

(event Input|ActionEvents|InputActionInteract
  (params (Key :type Key%20Structure :default "None"))
  (:Pressed
    (bind _asmaster_interact (Utilities|Casting|CastToMaster_Interact (Variables|Default|GetObjectLookingAt)))
    (Default|InteractwithObject _asmaster_interact)))

(event Input|AxisEvents|InputAxisMoveForward
  (params (AxisValue :type Float%20%28single-precision%29))
  (Pawn|Input|AddMovementInput (Transformation|GetActorForwardVector) AxisValue false))

(event Input|AxisEvents|InputAxisMoveRight
  (params (AxisValue :type Float%20%28single-precision%29))
  (Pawn|Input|AddMovementInput (Transformation|GetActorRightVector) AxisValue false))

(event Input|AxisEvents|InputAxisLookHorizontal
  (params (AxisValue :type Float%20%28single-precision%29))
  (Pawn|Input|AddControllerYawInput AxisValue))

(event Input|AxisEvents|InputAxisLookVertical
  (params (AxisValue :type Float%20%28single-precision%29))
  (Pawn|Input|AddControllerPitchInput (* AxisValue -1.0)))

(event Input|KeyboardEvents|P
  (params (Key :type Key%20Structure :default "None"))
  (:Pressed
    (bind _isa (Utilities|FlowControl|FlipFlop)
      (:A
        _)
      (:B
        _))
    (Game|SetGamePaused _isa)
    (bind _returnvalue (UserInterface|CreateWidget "/Game/UI_Pause/Ui_Pause.Ui_Pause_C"))
    (UserInterface|Viewport|AddtoViewport _returnvalue 0)))

(event Input|KeyboardEvents|Escape
  (params (Key :type Key%20Structure :default "None"))
  (:Pressed
    (bind _isa (Utilities|FlowControl|FlipFlop)
      (:A
        _)
      (:B
        _))
    (Game|SetGamePaused _isa)
    (bind _returnvalue (UserInterface|CreateWidget "/Game/UI_Pause/Ui_Pause.Ui_Pause_C"))
    (UserInterface|Viewport|AddtoViewport _returnvalue 0)))

(fn ConstructionScript)