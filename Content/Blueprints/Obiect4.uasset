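; Interactable object that opens the fifth question widget (Intrebarea5) as one step in an ordered find-the-objects progression.
; InteractwithObject acts only when the "Found" stat equals 4, with a DoOnce limiting it to a single trigger.
; It feeds a FlipFlop into the game pause state, sets game-only input with a visible cursor, shows the widget and increments "Found".
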(event EventInteractwithObject
  (bind _returnvalue (Game|GetPlayerController 0))
  (bind _value (CallFunction|ReadStat "Found"))
  (if (== _value 4)
    (Utilities|FlowControl|DoOnce false
      (:Completed
        (bind _isa (Utilities|FlowControl|FlipFlop)
          (:A
            _)
          (:B
            _))
        (Game|SetGamePaused _isa)
        (Input|SetInputModeGameOnly _returnvalue)
        (Variables|/Script/Engine.PlayerController|SetbShowMouseCursor _returnvalue true)
        (bind _returnvalue_2 (UserInterface|CreateWidget "/Game/Intrebari+Locatie/Intrebarea5/Intrebarea5.Intrebarea5_C"))
        (UserInterface|Viewport|AddtoViewport _returnvalue_2 0)
        (CallFunction|AddStat "Found" 1)))))

(fn ConstructionScript
  (|CallParentFunction))